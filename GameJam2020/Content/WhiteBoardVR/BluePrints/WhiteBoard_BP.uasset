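; VR whiteboard actor that shows a render target on its mesh for pens to draw on and erase.
; Dynamic marker and eraser materials stamp hit UVs into the target, with settable ink colour and size, and an optional wipe at BeginPlay.
; DrawOn skips every third point, clearing its location list and printing a debug message; dot connecting is only an unwired stub.
; UV hits must be enabled in project settings.
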(event `self.ReceiveBeginPlay`
  ;[1 1 1] Create material instance at play, and wipes the board clean if Bool is True
  (bind _returnvalue (`KismetMaterialLibrary.CreateDynamicMaterialInstance` "/Game/WhiteBoardVR/Materials/WhiteBoardMarker_M.WhiteBoardMarker_M"))
  (set `self.WhiteboardMarker_MI` _returnvalue)
  (bind _returnvalue_2 (`KismetMaterialLibrary.CreateDynamicMaterialInstance` "/Game/WhiteBoardVR/Materials/WhiteBoardMarker_M.WhiteBoardMarker_M"))
  (set `self.WhiteboardMarker_2_MI` _returnvalue_2)
  (bind _returnvalue_3 (`KismetMaterialLibrary.CreateDynamicMaterialInstance` "/Game/WhiteBoardVR/Materials/WhiteBoardEraser_M.WhiteBoardEraser_M"))
  (set `self.WhiteBoard Eraser MI` _returnvalue_3)
  (if (`self.WipeBoard`)
    (`KismetRenderingLibrary.ClearRenderTarget2D` (`self.RenderTarget_Ref`))))

(event `Draw On`
  (params (`Location To Draw` :type "Vector2D Structure"))
  (bind _drawlocations (`self.DrawLocations`))
  (bind _whiteboardmarker_mi (`self.WhiteboardMarker_MI`))
  ;[1 1 1] Draws to render target - Requires UV hits enabled in project settings
  (`KismetArrayLibrary.Array_Add` _drawlocations `Location To Draw`)
  (`/Engine/EditorBlueprintResources/StandardMacros.CompareInt` (`KismetArrayLibrary.Array_Length` _drawlocations) 3
    (:`==`
      (`KismetArrayLibrary.Array_Clear` _drawlocations)
      (`KismetSystemLibrary.PrintString` "Connecting Dots!"))
    (:`<`
      (`MaterialInstanceDynamic.SetVectorParameterValue` _whiteboardmarker_mi "DrawLocation" (`KismetMathLibrary.Conv_VectorToLinearColor` (`KismetMathLibrary.Conv_Vector2DToVector` `Location To Draw`)))
      (`KismetRenderingLibrary.DrawMaterialToRenderTarget` (`self.RenderTarget_Ref`) _whiteboardmarker_mi))))

(event `/Game/WhiteBoardVR/VirtualRealityBP/Blueprints/PickupActorInterface.Draw`)

(event `/Game/WhiteBoardVR/VirtualRealityBP/Blueprints/PickupActorInterface.Dont Draw`
  (`KismetSystemLibrary.PrintString` " DONT FUCKIN DRAW"))

(event `Erase`
  (params (`Location to Draw` :type "Vector2D Structure"))
  (bind _whiteboard_eraser_mi (`self.WhiteBoard Eraser MI`))
  ;[1 1 1] Erases from render target - Requires UV hits enabled in project settings
  (`MaterialInstanceDynamic.SetVectorParameterValue` _whiteboard_eraser_mi "DrawLocation" (`KismetMathLibrary.Conv_VectorToLinearColor` (`KismetMathLibrary.Conv_Vector2DToVector` `Location to Draw`)))
  (`KismetRenderingLibrary.DrawMaterialToRenderTarget` (`self.RenderTarget_Ref`) _whiteboard_eraser_mi))

(event `Set Colour`
  (params (InkColour :type "LinearColor Structure"))
  ;[1 0.06014 0] Sets the current draw colour to match pen held - Called in WhiteBoardPen_BP
  (`MaterialInstanceDynamic.SetVectorParameterValue` (`self.WhiteboardMarker_MI`) "InkColour" InkColour))

(event `Set Size`
  (params (`Draw Size` :type "Float (double-precision)"))
  (`MaterialInstanceDynamic.SetScalarParameterValue` (`self.WhiteboardMarker_MI`) "DrawSize" `Draw Size`))

(fn `UserConstructionScript`
  (bind _whiteboard (`self.WhiteBoard`))
  (bind _returnvalue (`PrimitiveComponent.CreateDynamicMaterialInstance` _whiteboard 0 "/Game/WhiteBoardVR/Materials/WhiteBoard_M.WhiteBoard_M" "None"))
  (`MaterialInstanceDynamic.SetTextureParameterValue` _returnvalue "RenderTargetToUse" (`self.RenderTarget_Ref`))
  (`PrimitiveComponent.SetMaterial` _whiteboard 0 _returnvalue))