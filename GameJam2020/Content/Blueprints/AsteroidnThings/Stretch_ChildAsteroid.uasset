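; Asteroid child Blueprint that plays a tick-driven stretching animation before spawning its dependents.
; BeginPlay records the base size, runs the parent setup, calls SetMasterVel and holds Tick off for about two seconds.
; A tick counter then stages non-uniform scaling: stretch along Z, shrink back, stretch along Y, then call SpawnDependents with 2BSpawned.
; Scaling compounds per frame, so timing follows frame rate.
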(event `self.ReceiveBeginPlay`
  (`self.SetActorTickEnabled` false)
  (`KismetSystemLibrary.Delay` 0.01)
  (set `self.StretchedSize` (`self.Size`))
  (`parent.ReceiveBeginPlay`)
  (`self.Set Master Vel` false)
  (`KismetSystemLibrary.Delay` 2.0)
  (`self.SetActorTickEnabled` true))

(event `self.ReceiveTick`
  (params (DeltaSeconds :type "Float (single-precision)"))
  (bind _size (`self.Size`))
  (bind _tick_counter (`self.Tick Counter`))
  (bind _size_2 (`self.Size`))
  (`/Engine/EditorBlueprintResources/StandardMacros.IncrementInt` (`self.Tick Counter`)
    (:`  `
      (`/Game/Blueprints/MacroLibrary.If3Condition` (< _tick_counter 20) (< _tick_counter 40) (< _tick_counter 55)
        (:`If 1`
          (set `self.StretchedSize` (* (`self.StretchedSize`) 1.05))
          (`self.SetActorScale3D` (`KismetMathLibrary.MakeVector` _size_2 _size_2 (`self.StretchedSize`)) :!label _label))
        (:`Else if 2`
          (set `self.StretchedSize` (/ (`self.StretchedSize`) 1.05))
          (goto _label))
        (:`Else if 3`
          (bind _output_get (set `self.StretchedSize` (* (`self.StretchedSize`) 1.05)))
          (`self.SetActorScale3D` (`KismetMathLibrary.MakeVector` _size _output_get _size)))
        (:`Else`
          (`self.Spawn Dependents` (`self.2BSpawned`)))))))

(fn `UserConstructionScript`
  (`parent.UserConstructionScript`))