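; Child asteroid Blueprint that moves every tick and changes velocity after its first overlap.
; On BeginPlay it runs the parent logic and location setup, then holds ticking off for a short delay before setting the master velocity and arming collision.
; The first overlap once armed disarms it, waits CollideDelay, then switches to EndingVelocity and reapplies the master velocity.
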(event `self.ReceiveBeginPlay`
  (`parent.ReceiveBeginPlay`)
  (`self.SetActorTickEnabled` false)
  (`self.Location Setup`)
  (`KismetSystemLibrary.Delay` 2.0)
  (`self.SetActorTickEnabled` true)
  (`self.Set Master Vel` false)
  (set `self.Ready to Collide` true))

(event `self.ReceiveActorBeginOverlap`
  (params (OtherActor :type "Actor Object Reference"))
  (if (`self.Ready to Collide`)
    (set `self.Ready to Collide` false)
    (`KismetSystemLibrary.Delay` (`self.Collide Delay`))
    (set `self.Velocity` (`self.Ending Velocity`))
    (`self.Set Master Vel` false)))

(event `self.ReceiveTick`
  (params (DeltaSeconds :type "Float (single-precision)"))
  (`self.Move` DeltaSeconds))

(fn `UserConstructionScript`
  (`parent.UserConstructionScript`))