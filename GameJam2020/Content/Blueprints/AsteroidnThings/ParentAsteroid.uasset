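; Base asteroid actor that registers itself with BP_XRU_GameInstance and takes its size, red/blue/purple material and left/center/right lane from its variables.
; Move steps it along Y by velocity and despawns it outside the play range.
; SpawnDependents replaces it with still or moving child asteroids, chosen by velocity.
; SetMasterVel publishes velocity to the game instance per color, and Despawn writes a sentinel there before deregistering and destroying the actor.
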(event `self.ReceiveBeginPlay`
  (bind _sphere (`self.Sphere`))
  (bind _size (`self.Size`))
  (`self.Add Self to Array`)
  (`KismetSystemLibrary.Delay` 0.01)
  (`self.SetActorScale3D` (`KismetMathLibrary.MakeVector` _size _size _size))
  ;[1 1 1] Color Setup
  (`self.ColorIf`
    (:`If Red`
      (`PrimitiveComponent.SetMaterial` _sphere 0 "/Game/Blueprints/AsteroidnThings/RedMaterial.RedMaterial"))
    (:`If Blue`
      (`PrimitiveComponent.SetMaterial` _sphere 0 "/Game/Blueprints/AsteroidnThings/BlueMaterial.BlueMaterial"))
    (:`If Purple`
      (`PrimitiveComponent.SetMaterial` _sphere 0 "/Game/Blueprints/AsteroidnThings/PurpleMaterial.PurpleMaterial"))))

(fn `Add Self to Array`
  (bind _asbp_xru_game_instance (cast `/Game/LiamWorkspace/BluePrints/BP_XRU_GameInstance` (`GameplayStatics.GetGameInstance`)))
  (`KismetArrayLibrary.Array_Add` (`/Game/LiamWorkspace/BluePrints/BP_XRU_GameInstance.PresentAsteroids` _asbp_xru_game_instance) self))

(fn `Delete Runaways`
  (bind (_returnvalue_x _returnvalue_y) (`KismetMathLibrary.BreakVector` (`self.K2_GetActorLocation`)))
  (if (not (`KismetMathLibrary.InRange_FloatFloat` _returnvalue_y -8100.0 8100.0))
    (`self.Despawn`)))

(fn `Despawn`
  (`self.Set Master Vel` true)
  (bind _asbp_xru_game_instance (cast `/Game/LiamWorkspace/BluePrints/BP_XRU_GameInstance` (`GameplayStatics.GetGameInstance`)))
  (bind _returnvalue (`KismetArrayLibrary.Array_RemoveItem` (`/Game/LiamWorkspace/BluePrints/BP_XRU_GameInstance.PresentAsteroids` _asbp_xru_game_instance) self))
  (if (not _returnvalue)
    (`KismetSystemLibrary.PrintString` "Removal from array didn't work"))
  (`self.K2_DestroyActor`))

(fn `Location Setup`
  (`self.SideIf`
    (:`If Left`
      (set `self.Starting Location` (`self.Default Left`)))
    (:`If Center`
      (set `self.Starting Location` (`self.Default Center`)))
    (:`If Right`
      (set `self.Starting Location` (`self.Default Right`))))
  (`self.K2_SetActorLocationAndRotation` (`self.Starting Location`)))

(fn `Move`
  (params (`Tick Length` :type "Float (double-precision)"))
  (bind (_returnvalue_x _returnvalue_y) (`KismetMathLibrary.BreakVector` (`self.K2_GetActorLocation`)))
  (bind (_starting_location_x _starting_location_y _starting_location_z) (`KismetMathLibrary.BreakVector` (`self.Starting Location`)))
  (`SceneComponent.K2_SetWorldLocationAndRotation` :`self` (`self.DefaultSceneRoot`) :`NewLocation` (`KismetMathLibrary.MakeVector` _starting_location_x (+ _returnvalue_y (* `Tick Length` (* -1 (`self.Velocity`)))) _starting_location_z))
  (`self.Delete Runaways`))

(fn `Set Master Vel`
  (params (Null :type Boolean))
  (bind _temp_float (`self.Temp Float`))
  (if Null
    (set `self.Temp Float` -57000.601563)
    (else
      (set `self.Temp Float` (`self.Velocity`))))
  (bind _asbp_xru_game_instance (cast `/Game/LiamWorkspace/BluePrints/BP_XRU_GameInstance` (`GameplayStatics.GetGameInstance`)))
  (`self.ColorIf`
    (:`If Red`
      (set `/Game/LiamWorkspace/BluePrints/BP_XRU_GameInstance.VelRed` _temp_float _asbp_xru_game_instance))
    (:`If Blue`
      (set `/Game/LiamWorkspace/BluePrints/BP_XRU_GameInstance.VelBlue` _temp_float _asbp_xru_game_instance))
    (:`If Purple`
      (set `/Game/LiamWorkspace/BluePrints/BP_XRU_GameInstance.VelPurple` _temp_float _asbp_xru_game_instance))))

(fn `Spawn Dependents`
  (params (ToSpawn :type "Array of /Game/Blueprints/AsteroidnThings/End_Parameters Structure"))
  (bind _returnvalue (`SceneComponent.K2_GetComponentLocation` (`self.DefaultSceneRoot`)))
  (for _array_element ToSpawn
    (if (== 0.0 (`.Velocity_8_75FB7C5748D5D53FC930939AA059A1C9` (break `/Game/Blueprints/AsteroidnThings/End_Parameters` _array_element)))
      (`|SpawnActorFromClass` "/Game/Blueprints/AsteroidnThings/EndStill_ChildAsteroid.EndStill_ChildAsteroid_C" (`KismetMathLibrary.MakeTransform` _returnvalue) "Undefined" "OverrideRootScale" (break `/Game/Blueprints/AsteroidnThings/End_Parameters` _array_element) (`.Size_2_1328DE5748C6DCBD72E52CBD2D6039E2` (break `/Game/Blueprints/AsteroidnThings/End_Parameters` _array_element)) (`.Color_13_596783044EF0AADD4FB912942933EF88` (break `/Game/Blueprints/AsteroidnThings/End_Parameters` _array_element)) (`.Velocity_8_75FB7C5748D5D53FC930939AA059A1C9` (break `/Game/Blueprints/AsteroidnThings/End_Parameters` _array_element)) (`.Side_12_DF9A8E0947B0A486A0872988B212FD00` (break `/Game/Blueprints/AsteroidnThings/End_Parameters` _array_element)) null)
      (else
        (`|SpawnActorFromClass` "/Game/Blueprints/AsteroidnThings/EndMoving_ChildAsteroid.EndMoving_ChildAsteroid_C" (`KismetMathLibrary.MakeTransform` _returnvalue) "Undefined" "OverrideRootScale" (break `/Game/Blueprints/AsteroidnThings/End_Parameters` _array_element) (`.Size_2_1328DE5748C6DCBD72E52CBD2D6039E2` (break `/Game/Blueprints/AsteroidnThings/End_Parameters` _array_element)) (`.Color_13_596783044EF0AADD4FB912942933EF88` (break `/Game/Blueprints/AsteroidnThings/End_Parameters` _array_element)) (`.Velocity_8_75FB7C5748D5D53FC930939AA059A1C9` (break `/Game/Blueprints/AsteroidnThings/End_Parameters` _array_element)) (`.Side_12_DF9A8E0947B0A486A0872988B212FD00` (break `/Game/Blueprints/AsteroidnThings/End_Parameters` _array_element)) null))))
  (`self.Despawn`))

(fn `UserConstructionScript`)