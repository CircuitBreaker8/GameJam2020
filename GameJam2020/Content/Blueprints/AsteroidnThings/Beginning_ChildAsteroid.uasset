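; Child asteroid Blueprint that appears to act as a starting asteroid, relying on parent logic for setup and movement.
; On BeginPlay it disables Tick, runs location setup, waits two seconds, then starts moving, sets its master velocity and arms collision.
; While armed, the first overlap disarms it and, after a delay, spawns its dependents.
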(event `self.ReceiveBeginPlay`
  (`parent.ReceiveBeginPlay`)
  (`self.SetActorTickEnabled` false)
  (`self.Location Setup`)
  (`KismetSystemLibrary.Delay` 2.0)
  (`self.SetActorTickEnabled` true)
  (`self.Set Master Vel` false)
  (set `self.ReadyToCollide` true))

(event `self.ReceiveActorBeginOverlap`
  (params (OtherActor :type "Actor Object Reference"))
  (if (`self.ReadyToCollide`)
    (set `self.ReadyToCollide` false)
    (`KismetSystemLibrary.Delay` (`self.Collide Delay`))
    (`self.Spawn Dependents` (`self.2BSpawned`))))

(event `self.ReceiveTick`
  (params (DeltaSeconds :type "Float (single-precision)"))
  (`self.Move` DeltaSeconds))

(fn `UserConstructionScript`
  (`parent.UserConstructionScript`))